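; BP_Door is a key-locked door that opens when the first-person character overlaps its trigger box.
; The overlap checks the character's PickedUpKey flag; without the key, it plays a locked sound and shows a prompt.
; With the key, it plays a door sound, destroys the box and calls OpenDoor, whose timeline sets the mesh to a fixed yaw or roll rotation on update, without interpolation.
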(event `OpenDoor`
  (`Timeline|OpenDoorTimeline`
    (:`Update`
      (`SceneComponent.K2_SetRelativeRotation` (`self.hinged_door3_fbx`) (struct :`Yaw` -90.0) false false))))

(event `self.Box.OnComponentBeginOverlap`
  (params (OverlappedComponent :type "PrimitiveComponent Object Reference") (OtherActor :type "Actor Object Reference") (OtherComp :type "PrimitiveComponent Object Reference") (OtherBodyIndex :type Integer) (bFromSweep :type Boolean) (SweepResult :type "HitResult Structure (by ref)"))
  (bind _asbp_first_person_character (cast `/Game/FirstPerson/Blueprints/BP_FirstPersonCharacter` OtherActor))
  (if (`/Game/FirstPerson/Blueprints/BP_FirstPersonCharacter.PickedUpKey` _asbp_first_person_character)
    (`GameplayStatics.PlaySound2D` "/Game/Audio/Door.Door" 1.0 1.0 0.0 null null)
    (`ActorComponent.K2_DestroyComponent` (`self.Box`))
    (`self.OpenDoor`)
    (`KismetSystemLibrary.PrintString` "Door open")
    (else
      (`GameplayStatics.PlaySound2D` "/Game/Audio/LockedDoor.LockedDoor" 1.0 1.0 0.0 null null)
      (`KismetSystemLibrary.PrintText` "You need the key"))))

(fn `UserConstructionScript`)